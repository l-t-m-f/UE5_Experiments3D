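; Player controller that handles mouse-driven camera look and sets Game and UI input mode focused on the game mode's HUD at BeginPlay.
; An LMB press sets a Mouse array flag that gates both axes; no connected logic clears it.
; Mouse X adds yaw input to the player character.
; Mouse Y changes the BP_PlayableCharacter spring arm's pitch, unclamped, with roll and yaw fixed.
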(event `self.ReceiveBeginPlay`
  (bind _asbp_game_mode_default (cast `/Game/Blueprints/BP_GameModeDefault` (`GameplayStatics.GetGameMode`))
    (:`then`
      (`WidgetBlueprintLibrary.SetInputMode_GameAndUIEx` (`GameplayStatics.GetPlayerController` 0) (`/Game/Blueprints/BP_GameModeDefault.HUD` _asbp_game_mode_default) "DoNotLock" false))
    (:`CastFailed`
      (`KismetSystemLibrary.PrintString` "Error in BP_PlayerController: Wrong game mode class "))))

(event `InputAxisKey|MouseY`
  (params (AxisValue :type "Float (single-precision)"))
  (if (`|GetArrayItem` (`self.Mouse`))
    (bind _asbp_playable_character (cast `/Game/Blueprints/BP_PlayableCharacter` (`GameplayStatics.GetPlayerCharacter` 0)))
    (bind _output_get (set `self.CurrentPlayerCameraArm` (`/Game/Blueprints/BP_CharacterBase.SpringArm` _asbp_playable_character)))
    (bind (_returnvalue_roll _returnvalue_pitch) (`KismetMathLibrary.BreakRotator` (`SpringArmComponent.GetTargetRotation` _output_get)))
    (`SceneComponent.K2_SetRelativeRotation` _output_get (`KismetMathLibrary.MakeRotator` 0.0 (+ _returnvalue_pitch AxisValue) 90.0) false false)))

(event `InputAxisKey|MouseX`
  (params (AxisValue :type "Float (single-precision)"))
  (if (`|GetArrayItem` (`self.Mouse`))
    (`Pawn.AddControllerYawInput` (`GameplayStatics.GetPlayerCharacter` 0) AxisValue)))

(event `InputAction|LMB`
  (params (Key :type "Key Structure"))
  (:`Pressed`
    (`KismetArrayLibrary.Array_Set` (`self.Mouse`) 0 true)))

(fn `UserConstructionScript`)