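; BP_ReplacableWall is a wall that vanishes and can reappear recolored once the first-person player passes through it.
; Actor tags step from forward to backward triggers, arming the activation events; backward activation hides the wall.
; The exit volume marks the pass and re-arms only the backward tag, as the ShowOnFacing branch is empty.
; Forward or backward activation then restores visibility per ShowOnFacing/ShowOnNotFacing, setting Albedo from Color1 or Color2.
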(event `self.ReceiveBeginPlay`
  (set `self.Tags` (`|MakeArray` (`self.ForwardTriggers`))))

(event `/Game/Blueprints/Interfaces/BPI_TriggerForwardTrace.ForwardActivation`
  (bind (_color1_b _color1_g _color1_r) (break `Color` (`self.Color1`)))
  (if (`self.IsHidden`)
    (if (`self.IsPlayerPassedThru`)
      (if (`self.ShowOnFacing`)
        (`SceneComponent.SetVisibility` (`self.StaticMesh`) true false)
        (set `self.IsHidden` false)
        (`self.SetTag` "None")
        (`PrimitiveComponent.SetCollisionEnabled` (`self.ExitVolume`) "NoCollision")
        (`MeshComponent.SetVectorParameterValueOnMaterials` (`self.StaticMesh`) "Albedo" (`KismetMathLibrary.MakeVector` (`KismetMathLibrary.Conv_ByteToDouble` _color1_b) (`KismetMathLibrary.Conv_ByteToDouble` _color1_g) (`KismetMathLibrary.Conv_ByteToDouble` _color1_r)))))
    (else
      (`self.SetTag` (`self.BackwardTriggers`)))))

(event `/Game/Blueprints/Interfaces/BPI_TriggerBackwardTrace.BackwardActivation`
  (bind (_color2_b _color2_g _color2_r) (break `Color` (`self.Color2`)))
  (`self.SetTag` "None")
  (if (`self.IsHidden`)
    (if (`self.IsPlayerPassedThru`)
      (if (`self.ShowOnNotFacing`)
        (`SceneComponent.SetVisibility` (`self.StaticMesh`) true false)
        (set `self.IsHidden` false)
        (`self.SetTag` "None")
        (`PrimitiveComponent.SetCollisionEnabled` (`self.ExitVolume`) "NoCollision")
        (`MeshComponent.SetVectorParameterValueOnMaterials` (`self.StaticMesh`) "Albedo" (`KismetMathLibrary.MakeVector` (`KismetMathLibrary.Conv_ByteToDouble` _color2_b) (`KismetMathLibrary.Conv_ByteToDouble` _color2_g) (`KismetMathLibrary.Conv_ByteToDouble` _color2_r)))))
    (else
      (`SceneComponent.SetVisibility` (`self.StaticMesh`) false false)
      (set `self.IsHidden` true)
      (`PrimitiveComponent.SetCollisionEnabled` (`self.CollisionVolume`) "NoCollision"))))

(event `self.ExitVolume.OnComponentBeginOverlap`
  (params (OverlappedComponent :type "PrimitiveComponent Object Reference") (OtherActor :type "Actor Object Reference") (OtherComp :type "PrimitiveComponent Object Reference") (OtherBodyIndex :type Integer) (bFromSweep :type Boolean) (SweepResult :type "HitResult Structure (by ref)"))
  (cast `/Game/Blueprints/BP_FirstPersonCharacter` OtherActor
    (:`then`
      (set `self.IsPlayerPassedThru` true)
      (`PrimitiveComponent.SetCollisionEnabled` (`self.ExitVolume`) "NoCollision")
      (set `self.Tags` (`|MakeArray` "None" :!type "Name"))
      (if (`self.ShowOnNotFacing`)
        (`KismetArrayLibrary.Array_Add` (`self.Tags`) (`self.BackwardTriggers`)))
      (if (`self.ShowOnFacing`)
        _))
    (:`CastFailed`
      (`KismetSystemLibrary.PrintString` "Wrong player type" :!label _label))))

(event `self.CollisionVolume.OnComponentBeginOverlap`
  (params (OverlappedComponent :type "PrimitiveComponent Object Reference") (OtherActor :type "Actor Object Reference") (OtherComp :type "PrimitiveComponent Object Reference") (OtherBodyIndex :type Integer) (bFromSweep :type Boolean) (SweepResult :type "HitResult Structure (by ref)"))
  (cast `/Game/Blueprints/BP_FirstPersonCharacter` OtherActor
    (:`then`
      (set `self.IsPlayerPassedThru` false))
    (:`CastFailed`
      (goto _label))))

(fn `SetTag`
  (params (Tag :type Name))
  (set `self.Tags` (`|MakeArray` Tag)))

(fn `UserConstructionScript`)