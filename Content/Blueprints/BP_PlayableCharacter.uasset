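; BP_PlayableCharacter is the player-controlled character, adding movement input and HUD health feedback on top of its parent class.
; The AxisX and AxisY input events share one SetDeltaMove call that updates horizontal movement, with Z held at zero.
; Its TakeDamage override runs the parent logic, then finds the first top-level WBP_HUD and sets its health bar to the clamped ratio of the two Health values.
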(event `InputAxis|AxisX`
  (params (AxisValue :type "Float (single-precision)"))
  (`self.SetDeltaMove` (`KismetMathLibrary.MakeVector` AxisValue (stale `InputAxis|AxisY` AxisValue)) :!label _label))

(event `InputAxis|AxisY`
  (params (AxisValue :type "Float (single-precision)"))
  (goto _label))

(fn `TakeDamage`
  (params (InputPin :type Integer))
  (bind _health (`self.Health`))
  (`parent.TakeDamage` InputPin)
  (bind _foundwidgets (`WidgetBlueprintLibrary.GetAllWidgetsOfClass` "/Game/Blueprints/Widgets/WBP_HUD.WBP_HUD_C"))
  (`/Game/Blueprints/Widgets/WBP_Bars.SetHealth` (`/Game/Blueprints/Widgets/WBP_HUD.ValueBars` (`|GetArrayItem` _foundwidgets)) (`KismetMathLibrary.FClamp` (/ (`KismetMathLibrary.Conv_IntToDouble` (`|GetArrayItem` _health)) (`KismetMathLibrary.Conv_IntToDouble` (`|GetArrayItem` _health 1))))))

(fn `UserConstructionScript`)