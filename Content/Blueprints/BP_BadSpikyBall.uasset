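; BP_BadSpikyBall is a hazard actor that slides back and forth along the X axis and damages actors that overlap it.
; BeginPlay stores the root's starting relative location, and Tick offsets it by a shift that reverses direction after passing either Limit.
; The shift changes by RateOfChange each frame without delta time, so speed depends on frame rate.
; Overlaps pass the other actor to BPContactDamageComponent to deal damage.
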(event `self.ReceiveBeginPlay`
  (bind _returnvalue_location (`KismetMathLibrary.BreakTransform` (`SceneComponent.GetRelativeTransform` (`self.DefaultSceneRoot`))))
  (set `self.StartingLocation` _returnvalue_location))

(event `self.ReceiveTick`
  (params (DeltaSeconds :type "Float (single-precision)"))
  (bind _currentshift (`self.CurrentShift`))
  (bind _currentshift_2 (`self.CurrentShift`))
  (bind _rateofchange (`self.RateOfChange`))
  (bind _limit (`self.Limit`))
  (bind (_startinglocation_x _startinglocation_y _startinglocation_z) (`KismetMathLibrary.BreakVector` (`self.StartingLocation`)))
  (`SceneComponent.K2_SetRelativeLocation` (`self.DefaultSceneRoot`) (`KismetMathLibrary.MakeVector` (+ _startinglocation_x (`self.CurrentShift`)) _startinglocation_y _startinglocation_z) false false)
  (switch `string` (`self.Dir`)
    (:`Left`
      (if (>= _currentshift_2 (* _limit -1.0))
        (set `self.CurrentShift` (- _currentshift _rateofchange))
        (else
          (set `self.Dir` "Right"))))
    (:`Right`
      (if (<= _currentshift_2 _limit)
        (set `self.CurrentShift` (+ _currentshift _rateofchange))
        (else
          (set `self.Dir` "Left"))))))

(event `self.ReceiveActorBeginOverlap`
  (params (OtherActor :type "Actor Object Reference"))
  (`/Game/Blueprints/BP_ContactDamageComponent.IDealDamage` (`self.BP_ContactDamageComponent`) OtherActor))

(fn `UserConstructionScript`)