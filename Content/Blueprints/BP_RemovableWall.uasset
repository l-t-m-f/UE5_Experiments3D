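; BP_RemovableWall is a wall actor that is removed after a two-stage activation sequence.
; On BeginPlay it sets its tags to ForwardTriggers, and ForwardActivation swaps them to BackwardTriggers.
; BackwardActivation then sets the tag to None and destroys the actor, so the Tags array serves as the wall's current state.
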(event `self.ReceiveBeginPlay`
  (set `self.Tags` (`|MakeArray` (`self.ForwardTriggers`))))

(event `/Game/Blueprints/Interfaces/BPI_TriggerForwardTrace.ForwardActivation`
  (set `self.Tags` (`|MakeArray` (`self.BackwardTriggers`))))

(event `/Game/Blueprints/Interfaces/BPI_TriggerBackwardTrace.BackwardActivation`
  (set `self.Tags` (`|MakeArray` "None" :!type "Name"))
  (`self.K2_DestroyActor`))

(fn `UserConstructionScript`)