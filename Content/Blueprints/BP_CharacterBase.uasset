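; BP_CharacterBase is a base character Blueprint that provides movement, idle/walk animation and health.
; Each tick it feeds the DeltaMove vector, set through SetDeltaMove, into forward and right movement input.
; A two-state Animation switch plays idle or walk clips directly on the mesh, only when movement starts or stops.
; ITakeDamage subtracts damage from the first Health array element, which GetCurrentHealth returns.
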(event `self.ReceiveTick`
  (params (DeltaSeconds :type "Float (single-precision)"))
  (`self.DoMovement`)
  (`self.PlayAnimation`))

(event `/Game/Blueprints/BPI_DamageTaking.ITakeDamage`
  (params (DamageAmount :type Integer))
  (`self.TakeDamage` DamageAmount))

(fn `CheckIfMoving`
  (returns (Result :type Boolean))
  (bind (_deltamove_x _deltamove_y _deltamove_z) (`KismetMathLibrary.BreakVector` (`self.DeltaMove`)))
  (return (or (!= _deltamove_x 0.0) (!= _deltamove_y 0.0) (!= _deltamove_z 0.0))))

(fn `DoMovement`
  (bind (_deltamove_x _deltamove_y _deltamove_z) (`KismetMathLibrary.BreakVector` (`self.DeltaMove`)))
  (bind (_deltamove_x_2 _deltamove_y_2) (`KismetMathLibrary.BreakVector` (`self.DeltaMove`)))
  (if (or (!= _deltamove_x 0.0) (!= _deltamove_y 0.0) (!= _deltamove_z 0.0))
    (`self.AddMovementInput` (`self.GetActorForwardVector`) _deltamove_x_2)
    (`self.AddMovementInput` (`self.GetActorRightVector`) _deltamove_y_2)))

(fn `GetCurrentHealth`
  (returns (CurrentHealth :type Integer))
  (return (`|GetArrayItem` (`self.Health`))))

(fn `PlayAnimation`
  (bind _result (`self.CheckIfMoving`))
  (bind _mesh (`self.Mesh`))
  (switch `/Game/Blueprints/Enums/E_AnimNames` (`self.Animation`)
    (:`NewEnumerator0`
      (if _result
        (`SkeletalMeshComponent.PlayAnimation` _mesh "/Engine/Tutorial/SubEditors/TutorialAssets/Character/Tutorial_Walk_Fwd.Tutorial_Walk_Fwd" true)
        (set `self.Animation` "NewEnumerator1")))
    (:`NewEnumerator1`
      (if (not _result)
        (`SkeletalMeshComponent.PlayAnimation` _mesh "/Engine/Tutorial/SubEditors/TutorialAssets/Character/Tutorial_Idle.Tutorial_Idle" true)
        (set `self.Animation` "NewEnumerator0")))))

(fn `SetDeltaMove`
  (params (NewDeltaMove :type "Vector Structure"))
  (set `self.DeltaMove` NewDeltaMove))

(fn `TakeDamage`
  (params (InputPin :type Integer))
  (bind _health (`self.Health`))
  (`KismetArrayLibrary.Array_Set` _health 0 (- (`|GetArrayItem` _health) InputPin)))

(fn `UserConstructionScript`)